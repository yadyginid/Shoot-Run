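; BP_HealthComponent is an actor component that tracks its owner's health and death state.
; It binds to the owner's any-damage event on BeginPlay, subtracts damage while alive, prints the health, and fires update and death dispatchers.
; Every hit is also reported as an AI Perception damage event, with the owner's AI controller as the damaged actor and the damage causer as instigator.
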(event Custom|OnTakeAnyDamage_Event
  (params (DamagedActor :type Actor%20Object%20Reference) (Damage :type Float%20%28single-precision%29) (DamageType :type Damage%20Type%20Object%20Reference) (InstigatedBy :type Controller%20Object%20Reference) (DamageCauser :type Actor%20Object%20Reference))
  (bind _returnvalue (Components|GetOwner))
  (bind _returnvalue_2 (Transformation|GetActorLocation _returnvalue))
  (CallFunction|ApplyDamage Damage)
  (Utilities|IsValid _returnvalue
    (:Is%20Valid
      (Class|AISenseDamage|ReportDamageEvent (AI|GetAIController _returnvalue) DamageCauser Damage _returnvalue_2 _returnvalue_2 "None"))))

(event EventBeginPlay
  (EventDispatchers|AssignOnTakeAnyDamage (Components|GetOwner) (delegate Custom|OnTakeAnyDamage_Event)))

(fn ApplyDamage
  (params (Value :type Float%20%28double-precision%29))
  (if (not (Variables|Default|GetDead))
    (bind _output_get (Variables|Default|SetHealth (- (Variables|Default|GetHealth) Value)))
    (Default|CallOnUpdateHealth)
    (Development|PrintString (Utilities|String|Append "Health is: " (Utilities|String|ToString(Float) _output_get)))
    (if (<= _output_get 0.0)
      (Variables|Default|SetDead (<= _output_get 0.0))
      (Default|CallOnDead))))