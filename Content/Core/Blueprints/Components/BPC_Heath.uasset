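; Health component that tracks the health and alive state of the actor it is attached to.
; On BeginPlay it binds to the owner's OnTakeAnyDamage event and passes incoming damage to its Damage function.
; While alive, Damage subtracts from Health and prints the new value, then at zero or below clears Alive and broadcasts the Dead dispatcher.
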(event Custom|OnDamaged
  (params (DamagedActor :type Actor%20Object%20Reference) (Damage :type Float%20%28single-precision%29) (DamageType :type Damage%20Type%20Object%20Reference) (InstigatedBy :type Controller%20Object%20Reference) (DamageCauser :type Actor%20Object%20Reference))
  (CallFunction|Damage Damage))

(event EventBeginPlay
  (EventDispatchers|BindEventtoOnTakeAnyDamage (Components|GetOwner) (delegate Custom|OnDamaged)))

(fn Dead)

(fn Damage
  (params (Damage%20Amount :type Float%20%28double-precision%29))
  (if (Variables|Default|GetAlive)
    (bind _output_get (Variables|Default|SetHealth (- (Variables|Default|GetHealth) Damage%20Amount)))
    (Development|PrintString (Utilities|String|ToString(Float) _output_get))
    (if (<= _output_get 0.0)
      (Variables|Default|SetAlive false)
      (Default|CallOnDead))))