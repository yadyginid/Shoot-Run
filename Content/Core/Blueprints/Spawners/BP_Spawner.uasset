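; BP_Spawner is a spawner actor that creates BP_Enemy NPCs in front of itself, up to a maximum count.
; BeginPlay spawns immediately and starts a one-second timer that repeats if Looping is set.
; Each spawn event creates up to two enemies, incrementing a counter that is never decremented.
; SwitchLoop flips Looping without resetting the timer, and a test game-mode binding is left unconnected.
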(event Custom|SpawnNPC
  (bind _returnvalue (Transformation|GetActorLocation))
  (bind _returnvalue_2 (Transformation|GetActorForwardVector))
  (bind _returnvalue_3 (* _returnvalue_2 3e+02))
  (Utilities|FlowControl|Sequence
    (:then_0
      (if (< (Variables|Default|GetCount%20NPC) (Variables|Default|GetMax%20Count%20NPC))
        (Game|SpawnActorfromClass "/Game/Core/Blueprints/Character/Enemy/BP_Enemy.BP_Enemy_C" (Math|Conversions|ToTransform(Vector) (+ _returnvalue _returnvalue_3)) "AdjustIfPossibleButAlwaysSpawn" "MultiplyWithRoot" 0 0)
        (Math|Integer|IncrementInt (Variables|Default|GetCount%20NPC))))
    (:then_1
      (if (< (Variables|Default|GetCount%20NPC) (Variables|Default|GetMax%20Count%20NPC))
        (Game|SpawnActorfromClass "/Game/Core/Blueprints/Character/Enemy/BP_Enemy.BP_Enemy_C" (Math|Conversions|ToTransform(Vector) (+ _returnvalue_3 _returnvalue)) "AdjustIfPossibleButAlwaysSpawn" "MultiplyWithRoot" 0 0)
        (Math|Integer|IncrementInt (Variables|Default|GetCount%20NPC))))))

(event EventBeginPlay
  (CallFunction|SpawnNPC)
  (Utilities|Time|SetTimerbyEvent (delegate Custom|SpawnNPC) 1.0 (Variables|Default|GetLooping)))

(fn ConstructionScript)

(fn SwitchLoop
  (if (Variables|Default|GetLooping)
    (Variables|Default|SetLooping false)
    (else
      (Variables|Default|SetLooping true))))