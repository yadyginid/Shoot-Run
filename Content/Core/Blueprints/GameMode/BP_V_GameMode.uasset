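; BP_V_GameMode is a game mode that spawns BP_NPC actors, up to a maximum count.
; It spawns one on BeginPlay and another whenever its SpawnNPC event dispatcher fires.
; Each spawn increments the count, places the NPC at the world origin, randomly sets it as enemy or not, passes itself as Spawner and calls the NPC's TurnAILogic.
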(event Custom|SpawnNPC
  (CallFunction|SpawnActor))

(event EventBeginPlay
  (EventDispatchers|BindEventtoEventDispatcherSpawnNPC (delegate Custom|SpawnNPC))
  (CallFunction|SpawnActor))

(fn ConstructionScript)

(fn SpawnActor
  (if (< (Variables|Default|GetCurrentCountNPC) (Variables|Default|GetMaxCountNPC))
    (Variables|Default|SetCurrentCountNPC (+ (Variables|Default|GetCurrentCountNPC) 1))
    (bind _returnvalue (Game|SpawnActorfromClass "/Game/Core/Blueprints/NPC/BP_NPC.BP_NPC_C" (Math|Transform|MakeTransform "0, 0, 0") "Undefined" "MultiplyWithRoot" 0 0))
    (Variables|/Game/Core/Blueprints/NPC/BP_NPC.BP_NPC_C|SetIsEnemy _returnvalue (Math|Random|RandomBool))
    (Variables|/Game/Core/Blueprints/NPC/BP_NPC.BP_NPC_C|SetSpawner _returnvalue self)
    (Default|CallTurnAILogic _returnvalue)))