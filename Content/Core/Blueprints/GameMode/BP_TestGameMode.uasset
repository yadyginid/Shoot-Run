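; BP_TestGameMode is a test game mode that keeps spawning BP_Mob NPCs in front of the player.
; On BeginPlay it caches the BP_Player pawn, spawns immediately, then repeats on a looping timer.
; Each pass spawns up to two mobs at the same point ahead of the player, one with the default team and one with an alternate Team value.
; A running counter caps total spawns at MaxCountNPC and is never decremented here.
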(event Custom|SpawnNPC
  (bind __bp_player (Variables|Default|Get%20BP%20Player))
  (bind _returnvalue (Transformation|GetActorLocation __bp_player))
  (bind _returnvalue_2 (Transformation|GetActorForwardVector __bp_player))
  (bind _returnvalue_3 (* _returnvalue_2 3e+02))
  (Utilities|FlowControl|Sequence
    (:then_0
      (if (< (Variables|Default|GetCountNPC) (Variables|Default|GetMaxCountNPC))
        (Game|SpawnActorfromClass "/Game/Core/Blueprints/Character/Enemy/BP_Mob.BP_Mob_C" (Math|Conversions|ToTransform(Vector) (+ _returnvalue _returnvalue_3)) "AdjustIfPossibleButAlwaysSpawn" "MultiplyWithRoot" 0 "NewEnumerator0" 0)
        (Math|Integer|IncrementInt (Variables|Default|GetCountNPC))))
    (:then_1
      (if (< (Variables|Default|GetCountNPC) (Variables|Default|GetMaxCountNPC))
        (Game|SpawnActorfromClass "/Game/Core/Blueprints/Character/Enemy/BP_Mob.BP_Mob_C" (Math|Conversions|ToTransform(Vector) (+ _returnvalue_3 _returnvalue)) "AdjustIfPossibleButAlwaysSpawn" "MultiplyWithRoot" 0 "NewEnumerator1" 0)
        (Math|Integer|IncrementInt (Variables|Default|GetCountNPC))))))

(event EventBeginPlay
  (bind _asbp_player (Utilities|Casting|CastToBP_Player (Game|Player|GetPlayerPawn 0)))
  (Utilities|IsValid _asbp_player
    (:Is%20Valid
      (Variables|Default|Set%20BP%20Player _asbp_player)
      (CallFunction|SpawnNPC)
      (Utilities|Time|SetTimerbyEvent (delegate Custom|SpawnNPC) 5.0 true))))

(fn ConstructionScript)