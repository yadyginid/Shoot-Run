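; BP_BaseMob is a base enemy character with team and weapon components, a melee attack and a mine-planting action.
; BeginPlay initializes the team, and possession triggers a weapon check.
; Melee plays a smash montage that roots the mob and enables an overlap collision dealing fixed damage to other actors.
; Mine planting spawns a mine when its stoppable montage completes, then fires a finished dispatcher.
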(event OnComponentBeginOverlap(AttackCollision)
  (params (OverlappedComponent :type Primitive%20Component%20Object%20Reference) (OtherActor :type Actor%20Object%20Reference) (OtherComp :type Primitive%20Component%20Object%20Reference) (OtherBodyIndex :type Integer) (bFromSweep :type Boolean) (SweepResult :type Hit%20Result%20Structure%20%28by%20ref%29))
  (if (!= OtherActor self)
    (Game|Damage|ApplyDamage OtherActor 1e+01 0 0)))

(event Custom|ActivateMine
  (bind _returnvalue (Transformation|GetActorLocation))
  (bind (_x _y) (Math|Vector|BreakVector _returnvalue))
  (Animation|Montage|PlayMontage (Variables|Character|GetMesh) "/Game/Core/Blueprints/Player/Animations/A_ActivateMine_Montage.A_ActivateMine_Montage"
    (:OnCompleted
      (Game|SpawnActorfromClass (Variables|Default|GetMineClass) (Math|Transform|MakeTransform (Math|Vector|MakeVector _x _y 0.0) "0, 0, 0" "1.000000,1.000000,1.000000") "Undefined" "MultiplyWithRoot" self false 0)
      (Default|CallOnMineActivateFinished))))

(event Custom|StopActivateMine
  (Animation|Montage|MontageStop (Components|SkeletalMesh|GetAnimInstance (Variables|Character|GetMesh)) 0.0 0))

(event Custom|MelleAttack
  (bind _charactermovement (Variables|Character|GetCharacterMovement))
  (bind _attack_collision (Variables|Default|GetAttack%20Collision))
  (if (not (Variables|Default|GetisPlayAnimAttack))
    (Animation|Montage|PlayMontage (Variables|Character|GetMesh) "/Game/Core/Blueprints/Player/Animations/Smash_Montage.Smash_Montage"
      (:then
        (Collision|SetCollisionEnabled _attack_collision "QueryOnly")
        (Variables|/Script/Engine.CharacterMovementComponent|SetMaxWalkSpeed _charactermovement 0.0)
        (Variables|Default|SetisPlayAnimAttack true))
      (:OnCompleted
        (Collision|SetCollisionEnabled _attack_collision "NoCollision")
        (Variables|/Script/Engine.CharacterMovementComponent|SetMaxWalkSpeed _charactermovement 6e+02)
        (Variables|Default|SetisPlayAnimAttack false)))))

(event EventBeginPlay
  (|CallParentFunction)
  (Default|Init (Variables|Default|GetBP_TeamComponent) (Variables|Default|GetTeamId))
  (Collision|SetCollisionEnabled (Variables|Default|GetAttack%20Collision) "NoCollision"))

(event EventPossessed
  (params (NewController :type Controller%20Object%20Reference))
  (Default|CheckHasWeapon (Variables|Default|GetBP_WeaponComponent)))

(fn ConstructionScript)