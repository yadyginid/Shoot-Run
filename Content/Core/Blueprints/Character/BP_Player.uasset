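; BP_Player is the player character Blueprint, handling basic movement, turning and a death animation trigger.
; MoveForward and MoveRight axis events, marked as old, add movement input along control-rotation vectors, and Around adds controller yaw.
; The 1 key plays the AM_Dead montage.
; The Sprint axis event sets a Sprint flag to true without checking its value, and nothing here clears or reads it.
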(event Input|AxisEvents|InputAxisMoveForward
  (params (AxisValue :type Float%20%28single-precision%29))
  (bind _returnvalue (Pawn|GetControlRotation :!class /Script/Engine.Pawn))
  ;[0.15 0.15 0.15 0.5] Old move events
  (Pawn|Input|AddMovementInput (Math|Vector|GetForwardVector (Math|Rotator|MakeRotator (.roll _returnvalue) (.pitch _returnvalue) (.yaw _returnvalue))) AxisValue false))

(event Input|AxisEvents|InputAxisSprint
  (params (AxisValue :type Float%20%28single-precision%29))
  (Variables|Default|SetSprint true))

(event Input|AxisEvents|InputAxisMoveRight
  (params (AxisValue :type Float%20%28single-precision%29))
  (bind _returnvalue (Pawn|GetControlRotation :!class /Script/Engine.Pawn))
  ;[0.15 0.15 0.15 0.5] Old move events
  (Pawn|Input|AddMovementInput (Math|Vector|GetRightVector (Math|Rotator|MakeRotator 0.0 (.pitch _returnvalue) (.yaw _returnvalue))) AxisValue false))

(event Input|AxisEvents|InputAxisAround
  (params (AxisValue :type Float%20%28single-precision%29))
  (Pawn|Input|AddControllerYawInput AxisValue))

(event Input|KeyboardEvents|1
  (params (Key :type Key%20Structure :default "None"))
  (:Pressed
    (Animation|PlayAnimMontage "/Game/Core/Blueprints/Player/Animations/AM_Dead.AM_Dead" 1.0 "None")))

(fn ConstructionScript)