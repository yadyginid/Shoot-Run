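; BP_npcBase is a base NPC character that plays a taunt or greeting montage, then follows the player.
; On BeginPlay it caches the player and binds to the test game mode's EnemyEmotions event, which replays the animation.
; PlayAnim stops movement and picks the montage by IsEnemy.
; Montage completion starts an AIMoveTo toward the player, re-issued after a short delay on each success, with no failure handling.
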(event Custom|PlayAnim
  (Components|Movement|StopMovementImmediately (Variables|Character|GetCharacterMovement))
  (if (Variables|Default|GetIsEnemy)
    (Animation|Montage|PlayMontage (Variables|Character|GetMesh) "/Game/Core/Blueprints/Player/Animations/Emotions/AM_Taunt.AM_Taunt"
      (:OnCompleted
        (CallFunction|MovetoPlayer)))
    (else
      (Animation|Montage|PlayMontage (Variables|Character|GetMesh) "/Game/Core/Blueprints/Player/Animations/Emotions/AM_Hello.AM_Hello"
        (:OnCompleted
          (CallFunction|MovetoPlayer))))))

(event Custom|PlayerOrder
  (CallFunction|PlayAnim))

(event Custom|MoveToPlayer
  (AI|AIMoveTo self "0, 0, 0" (Variables|Default|GetBP%20Player) 2e+01 false :!label _label
    (:OnSuccess
      (Utilities|FlowControl|Delay 0.2)
      (goto _label))))

(event EventBeginPlay
  (bind _asbp_player_child (Utilities|Casting|CastToBP_Player_Child (Game|GetPlayerCharacter 0)))
  (Utilities|IsValid _asbp_player_child
    (:Is%20Valid
      (bind _output_get (Variables|Default|SetBP%20Player _asbp_player_child))
      (Development|PrintString (Utilities|GetDisplayName _output_get))
      (bind _asbp_test_game_mode (Utilities|Casting|CastToBP_TestGameMode (Game|GetGameMode)))
      (EventDispatchers|BindEventtoEventEnemyEmotions _asbp_test_game_mode (delegate Custom|PlayerOrder))
      (CallFunction|PlayAnim))))

(fn ConstructionScript)