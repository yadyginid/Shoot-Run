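; Player character Blueprint with lethal melee hits and sprint support.
; Characters other than itself that begin overlapping the melee collision take very high fixed damage, and the 1 key calls Restart on the FFA game mode.
; Sprint functions set a flag and swap max walk speed, while CanSprint rules out rightward or backward movement; none are called within this file.
; TryInteract is an empty stub.
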(event OnComponentBeginOverlap(OverlapMeleeCollision)
  (params (OverlappedComponent :type Primitive%20Component%20Object%20Reference) (OtherActor :type Actor%20Object%20Reference) (OtherComp :type Primitive%20Component%20Object%20Reference) (OtherBodyIndex :type Integer) (bFromSweep :type Boolean) (SweepResult :type Hit%20Result%20Structure%20%28by%20ref%29))
  (Utilities|IsValid OtherActor
    (:Is%20Valid
      (if (!= OtherActor self)
        (bind _ascharacter (Utilities|Casting|CastToCharacter OtherActor))
        (Game|Damage|ApplyDamage _ascharacter 1e+03 0 0)))))

(event Input|KeyboardEvents|1
  (params (Key :type Key%20Structure :default "None"))
  (:Pressed
    (bind _asbp_default_game_mode_ffa (Utilities|Casting|CastToBP_DefaultGameModeFFA (Game|GetGameMode)))
    (Default|Restart _asbp_default_game_mode_ffa)))

(fn ConstructionScript)

(fn CanSprint
  (return (and (not (Variables|Default|GetRightMove)) (not (Variables|Default|GetBack)))))

(fn TryInteract)

(fn Sprinton
  (Variables|Default|SetSprint true)
  (Variables|/Script/Engine.CharacterMovementComponent|SetMaxWalkSpeed (Variables|Character|GetCharacterMovement) (Variables|Default|GetSprintSpeed)))

(fn SprintOff
  (Variables|Default|SetSprint false)
  (Variables|/Script/Engine.CharacterMovementComponent|SetMaxWalkSpeed (Variables|Character|GetCharacterMovement) (Variables|Default|GetMax%20Walk%20Speed)))