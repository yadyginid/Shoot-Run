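; Player controller that turns Enhanced Input actions into movement and combat commands for the possessed BP_Player.
; On BeginPlay it adds the IMC_PlayerMovement mapping context and caches the pawn, which every action checks for validity.
; Move follows control rotation, Look applies yaw only, and sprint, fire and weapon switching forward to the pawn's functions.
; CanSprint is a stub returning false and is not used by the sprint input.
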(event Input|EnhancedActionEvents|EnhancedInputActionIA_Sprint
  (params (ActionValue :type Boolean) (ElapsedSeconds :type Float%20%28double-precision%29) (TriggeredSeconds :type Float%20%28double-precision%29) (InputAction :type Input%20Action%20Object%20Reference :default "/Game/Core/Input/Actions/IA_Sprint.IA_Sprint"))
  (bind _bp_player (Variables|Default|GetBP%20Player))
  (bind _bp_player_2 (Variables|Default|GetBP%20Player))
  ;[0.15 0.15 0.15 0.5] Enchanted Input Action
  (:Started
    (Utilities|IsValid _bp_player_2
      (:Is%20Valid
        (Default|Sprinton _bp_player_2))))
  (:Completed
    (Utilities|IsValid _bp_player
      (:Is%20Valid
        (Default|SprintOff _bp_player)))))

(event Input|EnhancedActionEvents|EnhancedInputActionIA_Move
  (params (ActionValue :type Vector%202D%20Structure) (ElapsedSeconds :type Float%20%28double-precision%29) (TriggeredSeconds :type Float%20%28double-precision%29) (InputAction :type Input%20Action%20Object%20Reference :default "/Game/Core/Input/Actions/IA_Move.IA_Move"))
  (bind _returnvalue (Pawn|GetControlRotation :!class /Script/Engine.Controller))
  (bind _returnvalue_2 (Pawn|GetControlRotation :!class /Script/Engine.Controller))
  (bind _bp_player (Variables|Default|GetBP%20Player))
  ;[0.15 0.15 0.15 0.5] Enchanted Input Action
  (Variables|Default|SetAction%20Value%20X (.x ActionValue))
  (Variables|Default|SetAction%20Value%20Y (.y ActionValue))
  (Variables|Default|SetBack (<= (.y ActionValue) 0.0))
  (Utilities|IsValid _bp_player
    (:Is%20Valid
      (Pawn|Input|AddMovementInput _bp_player (Math|Vector|GetForwardVector (Math|Rotator|MakeRotator (.roll _returnvalue_2) (.pitch _returnvalue_2) (.yaw _returnvalue_2))) (Variables|Default|GetAction%20Value%20Y) false)
      (Pawn|Input|AddMovementInput (Variables|Default|GetBP%20Player) (Math|Vector|GetRightVector (Math|Rotator|MakeRotator 0.0 (.pitch _returnvalue) (.yaw _returnvalue))) (Variables|Default|GetAction%20Value%20X) false))))

(event Input|EnhancedActionEvents|EnhancedInputActionIA_Look
  (params (ActionValue :type Vector%202D%20Structure) (ElapsedSeconds :type Float%20%28double-precision%29) (TriggeredSeconds :type Float%20%28double-precision%29) (InputAction :type Input%20Action%20Object%20Reference :default "/Game/Core/Input/Actions/IA_Look.IA_Look"))
  (bind _bp_player (Variables|Default|GetBP%20Player))
  ;[0.15 0.15 0.15 0.5] Enchanted Input Action
  ;;[0.15 0.15 0.15 0.5] Look Up
  (Utilities|IsValid _bp_player
    (:Is%20Valid
      (Pawn|Input|AddControllerYawInput _bp_player (.x ActionValue)))))

(event Input|EnhancedActionEvents|EnhancedInputActionIA_NextWeapon
  (params (ActionValue :type Boolean) (ElapsedSeconds :type Float%20%28double-precision%29) (TriggeredSeconds :type Float%20%28double-precision%29) (InputAction :type Input%20Action%20Object%20Reference :default "/Game/Core/Input/Actions/IA_NextWeapon.IA_NextWeapon"))
  ;[0.15 0.15 0.15 0.5] Enchanted Input Action
  (Utilities|IsValid (Variables|Default|GetBP%20Player)
    (:Is%20Valid
      (Default|ChangeWeapon (Variables|Default|GetBP%20Player)))))

(event Input|EnhancedActionEvents|EnhancedInputActionIA_Fire
  (params (ActionValue :type Boolean) (ElapsedSeconds :type Float%20%28double-precision%29) (TriggeredSeconds :type Float%20%28double-precision%29) (InputAction :type Input%20Action%20Object%20Reference :default "/Game/Core/Input/Actions/IA_Fire.IA_Fire"))
  (bind _bp_player (Variables|Default|GetBP%20Player))
  ;[0.15 0.15 0.15 0.5] Enchanted Input Action
  (Utilities|IsValid _bp_player
    (:Is%20Valid
      (Default|Fire _bp_player))))

(event EventBeginPlay
  (bind _self self)
  (bind _returnvalue (PlayerController|LocalPlayerSubsystems|GetEnhancedInputLocalPlayerSubsystem _self))
  (Utilities|IsValid _returnvalue
    (:Is%20Valid
      (Input|AddMappingContext _returnvalue "/Game/Core/Input/IMC_PlayerMovement.IMC_PlayerMovement" 0 "(bIgnoreAllPressedKeysUntilRelease=True,bForceImmediately=False,bNotifyUserSettings=False)")
      (bind _asbp_player (Utilities|Casting|CastToBP_Player (Pawn|GetControlledPawn)))
      (Variables|Default|SetBP%20Player _asbp_player))))

(fn ConstructionScript)

(fn CanSprint
  (return false))