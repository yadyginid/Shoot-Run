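; Felix player character Blueprint that handles axis-driven movement, yaw turning, sprinting and emote animations.
; Movement follows control rotation and sets forward and sideways flags, which allow sprint only when moving forward without strafing.
; Sprint switches the movement component's max walk speed between walk and sprint values.
; Three input actions play montages from an animation array, while the E key triggers a play-emotion event on the test game mode.
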(event Input|ActionEvents|InputActionPlayer_animation_one
  (params (Key :type Key%20Structure :default "None"))
  ;[0.15 0.15 0.15 0.5] Play Animations
  (:Pressed
    (Animation|PlayAnimMontage (Utilities|Array|Get(acopy) (Variables|Default|GetAnimationArr)) 1.0 "None")))

(event Input|ActionEvents|InputActionPlayer_animation_two
  (params (Key :type Key%20Structure :default "None"))
  ;[0.15 0.15 0.15 0.5] Play Animations
  (:Pressed
    (Animation|PlayAnimMontage (Utilities|Array|Get(acopy) (Variables|Default|GetAnimationArr) 1) 1.0 "None")))

(event Input|ActionEvents|InputActionPlayer_animation_three
  (params (Key :type Key%20Structure :default "None"))
  ;[0.15 0.15 0.15 0.5] Play Animations
  (:Pressed
    (Animation|PlayAnimMontage (Utilities|Array|Get(acopy) (Variables|Default|GetAnimationArr) 2) 1.0 "None")))

(event Input|AxisEvents|InputAxisSprint
  (params (AxisValue :type Float%20%28single-precision%29))
  (bind _charactermovement (Variables|Character|GetCharacterMovement))
  ;[0.15 0.15 0.15 0.5] Sprint
  (if (> AxisValue 0.0)
    (if (and (Variables|Default|GetisMovingForward?) (not (Variables|Default|GetisMovingSide?)))
      (Variables|Default|SetSprint true)
      (Variables|/Script/Engine.CharacterMovementComponent|SetMaxWalkSpeed _charactermovement (Variables|Default|GetMaxSprintSpeed))
      (else
        (Variables|Default|SetSprint false :!label _label)
        (Variables|/Script/Engine.CharacterMovementComponent|SetMaxWalkSpeed _charactermovement (Variables|Default|GetMaxWalkSpeed))))
    (else
      (goto _label))))

(event Input|AxisEvents|InputAxisMoveForward
  (params (AxisValue :type Float%20%28single-precision%29))
  (bind _returnvalue (Pawn|GetControlRotation :!class /Script/Engine.Pawn))
  ;[0.15 0.15 0.15 0.5] Old move events
  (Pawn|Input|AddMovementInput (Math|Vector|GetForwardVector (Math|Rotator|MakeRotator (.roll _returnvalue) (.pitch _returnvalue) (.yaw _returnvalue))) AxisValue false)
  ;[0.15 0.15 0.15 0.5] IsMovingForward?
  (if (> AxisValue 0.0)
    (Variables|Default|SetisMovingForward? true)
    (else
      (Variables|Default|SetisMovingForward? false))))

(event Input|AxisEvents|InputAxisMoveRight
  (params (AxisValue :type Float%20%28single-precision%29))
  (bind _returnvalue (Pawn|GetControlRotation :!class /Script/Engine.Pawn))
  ;[0.15 0.15 0.15 0.5] Old move events
  (Pawn|Input|AddMovementInput (Math|Vector|GetRightVector (Math|Rotator|MakeRotator 0.0 (.pitch _returnvalue) (.yaw _returnvalue))) AxisValue false)
  ;[0.15 0.15 0.15 0.5] IsMovingSide?
  (if (== AxisValue 0.0)
    (Variables|Default|SetisMovingSide? false)
    (else
      (Variables|Default|SetisMovingSide? true))))

(event Input|AxisEvents|InputAxisAround
  (params (AxisValue :type Float%20%28single-precision%29))
  (Pawn|Input|AddControllerYawInput AxisValue))

(event Input|KeyboardEvents|E
  (params (Key :type Key%20Structure :default "None"))
  (:Pressed
    (Default|CallEventPlayEmotion (Variables|Default|GetBP%20Test%20Game%20Mode))))

(fn ConstructionScript)