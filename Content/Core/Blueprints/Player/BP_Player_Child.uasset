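; BP_Player_Child is a child player character Blueprint that adds fire animations and forward sprinting.
; The first and second weapon fire inputs each play their own montage from the WeaponAnimationsFire array.
; Sprint and a hard-wired W key set flags that raise CharacterMovement's MaxWalkSpeed only when both are held.
; Releasing either one while the other is still held restores walk speed.
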(event Input|ActionEvents|InputActionSprint
  (params (Key :type Key%20Structure :default "None"))
  (bind _charactermovement (Variables|Character|GetCharacterMovement))
  ;[0.15 0.15 0.15 0.5] Sprint
  (:Pressed
    (bind _output_get (Variables|Default|SetSprint true))
    (if (and _output_get (stale Input|KeyboardEvents|W _output_get))
      (Variables|/Script/Engine.CharacterMovementComponent|SetMaxWalkSpeed _charactermovement 9e+02)
      (else
        (Variables|/Script/Engine.CharacterMovementComponent|SetMaxWalkSpeed _charactermovement 6e+02 :!label _label))))
  (:Released
    (bind _output_get_2 (Variables|Default|SetSprint false))
    (if (or (stale Input|KeyboardEvents|W _output_get_2) _output_get_2)
      (goto _label))))

(event Input|ActionEvents|InputActionFireFirstWeapon
  (params (Key :type Key%20Structure :default "None"))
  (:Pressed
    (Animation|PlayAnimMontage (Utilities|Array|Get(acopy) (Variables|Default|GetWeaponAnimationsFire)) 1.0 "None")))

(event Input|ActionEvents|InputActionFireSecondWeapon
  (params (Key :type Key%20Structure :default "None"))
  (:Pressed
    (Animation|PlayAnimMontage (Utilities|Array|Get(acopy) (Variables|Default|GetWeaponAnimationsFire) 1) 1.0 "None")))

(event Input|KeyboardEvents|W
  (params (Key :type Key%20Structure :default "None"))
  (bind _charactermovement (Variables|Character|GetCharacterMovement))
  ;[0.15 0.15 0.15 0.5] Sprint
  (:Pressed
    (bind _output_get (Variables|Default|SetWcheck true))
    (if (and (stale Input|ActionEvents|InputActionSprint _output_get) _output_get)
      (Variables|/Script/Engine.CharacterMovementComponent|SetMaxWalkSpeed _charactermovement 9e+02)
      (else
        (Variables|/Script/Engine.CharacterMovementComponent|SetMaxWalkSpeed _charactermovement 6e+02 :!label _label))))
  (:Released
    (bind _output_get_2 (Variables|Default|SetWcheck false))
    (if (or _output_get_2 (stale Input|ActionEvents|InputActionSprint _output_get_2))
      (goto _label))))

(event Input|KeyboardEvents|P
  (params (Key :type Key%20Structure :default "None")))

(fn ConstructionScript
  (|CallParentFunction))