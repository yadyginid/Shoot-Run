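; BP_Mine is a trap weapon that explodes when a Character overlaps its MineOverlap component.
; On a valid overlap it applies BaseDamage to that character, spawns a big explosion emitter at its location and destroys itself.
; The owner triggers it only when CanApplySelfDamage is set; otherwise the owner's overlap is ignored.
; Damage goes only to the overlapping character, with no radial falloff.
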(event OnComponentBeginOverlap(MineOverlap)
  (params (OverlappedComponent :type Primitive%20Component%20Object%20Reference) (OtherActor :type Actor%20Object%20Reference) (OtherComp :type Primitive%20Component%20Object%20Reference) (OtherBodyIndex :type Integer) (bFromSweep :type Boolean) (SweepResult :type Hit%20Result%20Structure%20%28by%20ref%29))
  (Utilities|Casting|CastToCharacter OtherActor)
  (if (Variables|Default|GetCanApplySelfDamage)
    (Game|Damage|ApplyDamage OtherActor (Variables|Default|GetBase%20Damage) 0 0 :!label _label)
    (Effects|SpawnEmitteratLocation "/Game/Realistic_Starter_VFX_Pack_Vol2/Particles/Explosion/P_Explosion_Big_C.P_Explosion_Big_C" (Transformation|GetActorLocation))
    (Actor|DestroyActor)
    (elif (!= OtherActor (Components|GetOwner))
      (goto _label))))

(fn ConstructionScript)