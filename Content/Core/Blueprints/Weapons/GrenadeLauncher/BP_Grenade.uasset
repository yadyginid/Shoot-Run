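; BP_Grenade is the grenade actor for the grenade launcher, exploding on a timed fuse.
; On BeginPlay it greatly raises the static mesh's mass scale, then waits TimeToExplosion seconds.
; It then applies radial damage at its location, spawns an explosion particle effect, fires the RadialForce impulse and destroys itself.
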(event EventBeginPlay
  (bind _returnvalue (Transformation|GetActorLocation))
  (Class|PrimitiveComponent|SetMassScale (Variables|Default|GetStaticMesh) "None" 1e+04)
  (Utilities|FlowControl|Delay (Variables|Default|GetTimeToExplosion))
  (Game|Damage|ApplyRadialDamage 5e+01 _returnvalue 5e+02 0 0 0 0 false "ECC_Visibility")
  (Effects|SpawnEmitteratLocation "/Game/Realistic_Starter_VFX_Pack_Vol2/Particles/Explosion/P_Explosion_Big_B.P_Explosion_Big_B" _returnvalue)
  (Class|RadialForceComponent|FireImpulse (Variables|Default|GetRadialForce))
  (Utilities|IsValid self
    (:Is%20Valid
      (Actor|DestroyActor))))

(fn ConstructionScript)