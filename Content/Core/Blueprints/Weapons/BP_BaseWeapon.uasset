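; Base hitscan weapon that fires a laser from the muzzle socket along a short visibility line trace.
; BeginPlay caches the owning character's mesh and doubles base damage if player controller 0 exists, regardless of owner.
; Fire draws a Niagara beam to the impact or trace end, damages hit actors, activates BP_MobBase hit effects and decals non-characters.
; A random shot montage on the character gates fire rate, re-enabling firing on completion.
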(event Custom|ShowEffects)

(event Custom|PlayeFireAnimation
  (bind _arrshotanimations (Variables|Default|GetArrShotAnimations))
  (Utilities|IsValid (Variables|Default|GetMesh)
    (:Is%20Valid
      (Animation|Montage|PlayMontage (Variables|Default|GetMesh) (Utilities|Array|Get(acopy) _arrshotanimations (Math|Random|RandomIntegerinRange 0 (- (Utilities|Array|Length _arrshotanimations) 1)))
        (:OnCompleted
          (Variables|Default|SetCanFire true))))))

(event Custom|Fire
  (bind _returnvalue (Components|GetOwner))
  (bind _skeletalmesh (Variables|Default|GetSkeletalMesh))
  (if (Variables|Default|GetCanFire)
    (Variables|Default|SetCanFire false)
    (Variables|Default|SetStartVector (Transformation|GetSocketLocation _skeletalmesh "Muzzle"))
    (Variables|Default|SetEndVector (* (Math|Vector|GetForwardVector (Transformation|GetSocketRotation _skeletalmesh "Muzzle")) 1000))
    (Variables|Default|SetHitVector (+ (Variables|Default|GetStartVector) (Variables|Default|GetEndVector)))
    (bind _outhit (Collision|LineTraceByChannel (Variables|Default|GetStartVector) (+ (Variables|Default|GetStartVector) (Variables|Default|GetEndVector)) "TraceTypeQuery1" false (Utilities|Array|MakeArray (Components|GetOwner)) "None"))
    (CallFunction|PlayeFireAnimation)
    (Variables|Default|SetHit%20Actor (.HitActor (Collision|BreakHitResult _outhit)))
    (CallFunction|PlayFireNiagara (Math|Vector|SelectVector (.ImpactPoint (Collision|BreakHitResult _outhit)) (Variables|Default|GetHitVector) (.bBlockingHit (Collision|BreakHitResult _outhit))))
    (if (.bBlockingHit (Collision|BreakHitResult _outhit))
      (Utilities|IsValid (Variables|Default|GetHit%20Actor)
        (:Is%20Valid
          (Game|Damage|ApplyDamage (Variables|Default|GetHit%20Actor) (Variables|Default|GetBase%20Damage) (Game|GetInstigatorController _returnvalue) _returnvalue)
          (CallFunction|PlayHitNiagaraEffects)
          (Utilities|Casting|CastToCharacter (Variables|Default|GetHit%20Actor)
            (:CastFailed
              (CallFunction|SpawnDecal _outhit))))))))

(event EventBeginPlay
  (bind _returnvalue (Game|GetPlayerController 0))
  (Development|PrintString "begin play")
  (bind _ascharacter (Utilities|Casting|CastToCharacter (Components|GetOwner)))
  (bind _output_get (Variables|Default|SetCharacter _ascharacter))
  (Variables|Default|SetMesh (Variables|/Script/Engine.Character|GetMesh _output_get))
  ;[0.15 0.15 0.15 0.5] More damage for player
  (Utilities|IsValid _returnvalue
    (:Is%20Valid
      (Variables|Default|SetPlayerController _returnvalue)
      (Variables|Default|SetBase%20Damage (* (Variables|Default|GetBase%20Damage) 2.0)))))

(event EventEndPlay
  (params (EndPlayReason :type EEndPlayReason%20Enum :default "Destroyed"))
  (Development|PrintString "end play"))

(fn ConstructionScript)

(fn ResetFire
  (Variables|Default|SetCanFire true))

(fn SpawnDecal
  (params (HitResult :type Hit%20Result%20Structure))
  (bind (_bblockinghit _binitialoverlap _time _distance _location _impactpoint _normal _impactnormal) (Collision|BreakHitResult HitResult))
  (Rendering|Decal|SpawnDecalatLocation "/Game/Effects/Materials/Weapon/M_Impact_Decal.M_Impact_Decal" "100.000000,100.000000,100.000000" _impactpoint (Math|Rotator|MakeRotfromX (* _impactnormal -1)) 3.0))

(fn PlayFireNiagara
  (params (TraceVector :type Vector))
  (bind _returnvalue (Niagara|SpawnSystemAttached "/Game/VFX/Trace/Rifle/NS_Laserbeam.NS_Laserbeam" (Variables|Default|GetSkeletalMesh) "Muzzle" (Transformation|GetSocketLocation (Variables|Default|GetSkeletalMesh) "Muzzle") "0, 0, 0" "KeepWorldPosition" false))
  (Niagara|SetNiagaraVariable(Vector3) _returnvalue "TraceTarget" TraceVector))

(fn PlayHitNiagaraEffects
  (bind _asbp_mob_base (Utilities|Casting|CastToBP_MobBase (Variables|Default|GetHit%20Actor)))
  (Components|Activation|Activate (Variables|/Game/Core/Blueprints/Character/Enemy/BP_MobBase.BP_MobBase_C|GetNS_Boom _asbp_mob_base) false))