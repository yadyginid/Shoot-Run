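; BP_NPC is a character that greets or threatens the player, walks over, then collapses.
; BeginPlay binds the TurnAILogic dispatcher, whose event plays an aggressive or hello montage depending on IsEnemy.
; Once the montage completes, both branches share an AI move to the player.
; On arrival it destroys its capsule, ragdolls the mesh and fires the SpawnNPC dispatcher on its Spawner, cast to BP_V_GameMode.
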(event Custom|Event%20TurnAILogic
  (bind _mesh (Variables|Character|GetMesh))
  (if (Variables|Default|GetIsEnemy)
    (Animation|Montage|PlayMontage _mesh (Variables|Default|GetAgressiveAnimMontage)
      (:OnCompleted
        _))
    (else
      (Animation|Montage|PlayMontage _mesh (Variables|Default|GetHelloAnimMontage)
        (:OnCompleted
          _))))
  (AI|AIMoveTo self "0, 0, 0" (Game|GetPlayerCharacter 0) 5.0 false
    (:OnSuccess
      (Components|DestroyComponent (Variables|Default|GetCapsuleComponent))
      (Physics|SetSimulatePhysics (Variables|Character|GetMesh) true)
      (bind _asbp_v_game_mode (Utilities|Casting|CastToBP_V_GameMode (Variables|Default|GetSpawner)))
      (Default|CallEventDispatcherSpawnNPC _asbp_v_game_mode))))

(event EventBeginPlay
  (EventDispatchers|BindEventtoTurnAILogic (delegate Custom|Event%20TurnAILogic)))

(fn ConstructionScript)