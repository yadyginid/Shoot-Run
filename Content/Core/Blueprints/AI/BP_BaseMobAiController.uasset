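; Base AI controller for mobs that sets up their behavior tree and tracks the player as a target.
; On possess, it initializes the BB_BaseAI blackboard with the mob and its two patrol points, then runs the behavior tree.
; AI perception updates write the sensed player to the Target key and clear it as soon as a player stimulus is lost.
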(event OnTargetPerceptionUpdated(AIPerception)
  (params (Actor :type Actor%20Object%20Reference) (Stimulus :type AI%20Stimulus%20Structure))
  (if (.bSuccessfullySensed (Utilities|Struct|BreakAIStimulus Stimulus))
    (bind _asbp_player (Utilities|Casting|CastToBP_Player Actor))
    (bind _output_get (Variables|Default|SetTargetActor _asbp_player))
    (AI|Components|Blackboard|SetValueasObject (Variables|Default|GetBlackboard%20Component) (Variables|Default|GetTarget) _output_get)
    (else
      (Utilities|Casting|CastToBP_Player Actor)
      (Variables|Default|SetTargetActor 0)
      (AI|Components|Blackboard|SetValueasObject (Variables|Default|GetBlackboard%20Component) (Variables|Default|GetTarget) 0))))

(event EventPossess
  (params (PossessedPawn :type Pawn%20Object%20Reference))
  (Utilities|IsValid (Class|BlackboardAssetProvider|GetBlackboardAsset (Variables|Default|GetBTAsset))
    (:Is%20Valid
      (bind _asbp_base_mob (Utilities|Casting|CastToBP_BaseMob (Pawn|GetControlledPawn)))
      (Variables|Default|SetBP%20Mob _asbp_base_mob)
      (bind _blackboardcomponent (Class|AIController|UseBlackboard "/Game/Core/Blueprints/AI/BT/BB_BaseAI.BB_BaseAI"))
      (Variables|Default|SetBlackboard%20Component _blackboardcomponent)
      (Utilities|IsValid _blackboardcomponent
        (:Is%20Valid
          (AI|Components|Blackboard|SetValueasObject (Variables|Default|GetBlackboard%20Component) (Variables|Default|GetPatrolPoint1) (Variables|/Game/Core/Blueprints/Character/Enemy/BP_BaseMob.BP_BaseMob_C|GetPatrolPoint1 (Variables|Default|GetBP%20Mob)))
          (AI|Components|Blackboard|SetValueasObject (Variables|Default|GetBlackboard%20Component) (Variables|Default|GetPatrolPoint2) (Variables|/Game/Core/Blueprints/Character/Enemy/BP_BaseMob.BP_BaseMob_C|GetPatrolPoint2 (Variables|Default|GetBP%20Mob)))
          (AI|Components|Blackboard|SetValueasObject (Variables|Default|GetBlackboard%20Component) (Variables|Default|GetOwnerBP_Mob) (Variables|Default|GetBP%20Mob))
          (AI|RunBehaviorTree (Variables|Default|GetBTAsset)))))))

(fn ConstructionScript)