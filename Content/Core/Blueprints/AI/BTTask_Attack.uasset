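; Behavior tree task that makes an AI-controlled BP_Mob attack its blackboard Target actor.
; It compares the distance to the target against a Distance threshold, calling the mob's melee attack within range and firing its weapon component otherwise.
; The task always finishes successfully right after triggering the action, or when the pawn cast or target check fails, without waiting for the attack to end.
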(event EventReceiveExecute
  (params (OwnerActor :type Actor%20Object%20Reference))
  (bind _asaicontroller (Utilities|Casting|CastToAIController OwnerActor))
  (bind _asbp_mob (Utilities|Casting|CastToBP_Mob (Pawn|GetControlledPawn _asaicontroller))
    (:then
      (Variables|Default|SetBP%20Mob _asbp_mob)
      (Variables|Default|SetBlackboard (AI|GetBlackboard OwnerActor))
      (bind _asactor (Utilities|Casting|CastToActor (AI|Components|Blackboard|GetValueasObject (Variables|Default|GetBlackboard) (Variables|Default|GetTarget)))
        (:then
          (Utilities|IsValid _asactor
            (:Is%20Valid
              (Variables|Default|SetTargetActor _asactor)
              (if (<= (Math|Vector|Distance(Vector) (Transformation|GetActorLocation (Variables|Default|GetBP%20Mob)) (Transformation|GetActorLocation (Variables|Default|GetTargetActor))) (Variables|Default|GetDistance))
                (Default|MelleAttack (Variables|Default|GetBP%20Mob))
                (AI|BehaviorTree|FinishExecute true)
                (else
                  (Default|Fire (Variables|/Game/Core/Blueprints/Character/Base/BP_CharacterBase.BP_CharacterBase_C|GetBP_WeaponComponent (Variables|Default|GetBP%20Mob)))
                  (AI|BehaviorTree|FinishExecute true))))
            (:Is%20Not%20Valid
              (AI|BehaviorTree|FinishExecute true :!label _label))))
        (:CastFailed
          (goto _label))))
    (:CastFailed
      (AI|BehaviorTree|FinishExecute true))))