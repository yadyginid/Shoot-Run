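; Base ammo pickup that adds ammunition to a character when it touches the pickup's sphere.
; On overlap, it casts the actor to BP_CharacterBaseKostin and adds NumAmmo to the TypeAmmo slot of the weapon component's NumAmmo array.
; It prints the new total, or an error if TypeAmmo exceeds the array bounds.
; The pickup is not destroyed or disabled afterwards, so every new overlap adds ammo again.
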(event OnComponentBeginOverlap(Sphere)
  (params (OverlappedComponent :type Primitive%20Component%20Object%20Reference) (OtherActor :type Actor%20Object%20Reference) (OtherComp :type Primitive%20Component%20Object%20Reference) (OtherBodyIndex :type Integer) (bFromSweep :type Boolean) (SweepResult :type Hit%20Result%20Structure%20%28by%20ref%29))
  (bind _asbp_character_base_kostin (Utilities|Casting|CastToBP_CharacterBaseKostin OtherActor))
  (Variables|Default|SetAs%20BP%20Character%20Base%20Kostin _asbp_character_base_kostin)
  (if (> (Utilities|Array|Length (Variables|/Game/Core/BP_Kostin/Component/BP_WeaponComponentKostin.BP_WeaponComponentKostin_C|GetNumAmmo (Variables|/Game/Core/BP_Kostin/Character/Base/BP_CharacterBaseKostin.BP_CharacterBaseKostin_C|GetBP_WeaponComponentKostin _asbp_character_base_kostin))) (Variables|Default|GetTypeAmmo))
    (Utilities|Array|SetArrayElem (Variables|/Game/Core/BP_Kostin/Component/BP_WeaponComponentKostin.BP_WeaponComponentKostin_C|GetNumAmmo (Variables|/Game/Core/BP_Kostin/Character/Base/BP_CharacterBaseKostin.BP_CharacterBaseKostin_C|GetBP_WeaponComponentKostin (Variables|Default|GetAs%20BP%20Character%20Base%20Kostin))) (Variables|Default|GetTypeAmmo) (+ (Utilities|Array|Get(acopy) (Variables|/Game/Core/BP_Kostin/Component/BP_WeaponComponentKostin.BP_WeaponComponentKostin_C|GetNumAmmo (Variables|/Game/Core/BP_Kostin/Character/Base/BP_CharacterBaseKostin.BP_CharacterBaseKostin_C|GetBP_WeaponComponentKostin (Variables|Default|GetAs%20BP%20Character%20Base%20Kostin))) (Variables|Default|GetTypeAmmo)) (Variables|Default|GetNumAmmo)))
    (Development|PrintString (Utilities|String|ToString(Integer) (Utilities|Array|Get(acopy) (Variables|/Game/Core/BP_Kostin/Component/BP_WeaponComponentKostin.BP_WeaponComponentKostin_C|GetNumAmmo (Variables|/Game/Core/BP_Kostin/Character/Base/BP_CharacterBaseKostin.BP_CharacterBaseKostin_C|GetBP_WeaponComponentKostin (Variables|Default|GetAs%20BP%20Character%20Base%20Kostin))) (Variables|Default|GetTypeAmmo))))
    (else
      (Development|PrintString "Error Type Ammo"))))

(event EventBeginPlay)

(event EventTick
  (params (DeltaSeconds :type Float%20%28single-precision%29)))

(fn ConstructionScript)