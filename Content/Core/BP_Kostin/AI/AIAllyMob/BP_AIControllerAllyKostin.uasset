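; AI controller for Kostin's ally mob that feeds its Blackboard a reference to the BP_CharacterBaseKostin actor.
; On possess it initializes the Blackboard and, if that succeeds, stores the first actor found of that class under an object key.
; SetWeapon sets a bool key to true and looks up the same character again to refresh the object key.
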(event EventPossess
  (params (PossessedPawn :type Pawn%20Object%20Reference))
  (bind _isinit (CallFunction|InitBlackboard))
  (if _isinit
    (bind _returnvalue (Actor|GetActorOfClass "/Game/Core/BP_Kostin/Character/Base/BP_CharacterBaseKostin.BP_CharacterBaseKostin_C"))
    (AI|Components|Blackboard|SetValueasObject (Variables|Default|GetBlackboard) (Variables|Default|GetKey%20Name) _returnvalue)))

(fn ConstructionScript)

(fn SetWeapon
  (AI|Components|Blackboard|SetValueasBool (Variables|Default|GetBlackboard) (Variables|Default|GetKey%20Name_0) true)
  (bind _returnvalue (Actor|GetActorOfClass "/Game/Core/BP_Kostin/Character/Base/BP_CharacterBaseKostin.BP_CharacterBaseKostin_C"))
  (AI|Components|Blackboard|SetValueasObject (Variables|Default|GetBlackboard) (Variables|Default|GetKey%20Name) _returnvalue))