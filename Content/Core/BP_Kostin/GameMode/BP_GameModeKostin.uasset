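; Game mode that holds weapon and ammo object pools and contains grid-based NPC spawning logic.
; Pooled actors snap-attach to a BP_ActorNULL actor; searches remove and return the first exact class match.
; GenNPC spawns BP_CharacterNPCKostin at grid positions advanced by GridFunction, clearing its timer at the NPC cap.
; The looping timer setup for GenNPC is unreachable and BeginPlay is empty, so this Blueprint never starts spawning itself.
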(event Custom|GenNPC
  (bind _griddistance (Variables|GridGenerate|GetGridDistance))
  ;[0.15 0.15 0.15 0.5] Grid Generate
  (if (> (Variables|GridGenerate|GetMaxNPC) (Variables|GridGenerate|GetNumNPC))
    (Variables|GridGenerate|SetNumNPC (+ (Variables|GridGenerate|GetNumNPC) 1))
    (Game|SpawnActorfromClass "/Game/Core/BP_Kostin/Character/NPC/BP_CharacterNPCKostin.BP_CharacterNPCKostin_C" (Math|Transform|MakeTransform (Math|Vector|MakeVector (+ (* (Variables|GridGenerate|GetNumGridSizeX) _griddistance) 1e+02) (+ (* _griddistance (Variables|GridGenerate|GetNumGridSizeY)) 1e+02) 0.0) "0, 0, 0" "1.000000,1.000000,1.000000") "Undefined" "MultiplyWithRoot" 0 0)
    (CallFunction|GridFunction)
    (else
      (Utilities|Time|ClearandInvalidateTimerbyHandle (Variables|GridGenerate|Get%20Handle)))))

(event EventBeginPlay)

(fn ConstructionScript)

(fn GridFunction
  (Variables|GridGenerate|SetNumGridSizeX (Math|Float|Truncate (.Remainder (Math|Float|Division(WholeandRemainder) (Math|Conversions|ToFloat(Integer) (+ (Variables|GridGenerate|GetNumGridSizeX) 1)) (Math|Conversions|ToFloat(Integer) (Variables|GridGenerate|GetGridSize))))))
  (Variables|GridGenerate|SetNumGridSizeY (/ (Variables|GridGenerate|GetNumNPC) (Variables|GridGenerate|GetGridSize))))

(fn FAddWeaponPool
  (params (OWeapon :type BP%20Weapon%20Base%20Kostin%20Object%20Reference))
  (Utilities|Array|Add (Variables|Default|GetArrayWeaponPool) OWeapon)
  (bind _returnvalue (Actor|GetActorOfClass "/Game/Core/BP_Kostin/Character/NPC/BP_ActorNULL.BP_ActorNULL_C"))
  (Transformation|AttachActorToActor OWeapon _returnvalue "None" "SnapToTarget" "SnapToTarget" "SnapToTarget" true))

(fn FSearchWeaponPool
  (params (CWeapon :type BP%20Weapon%20Base%20Kostin%20Class%20Reference))
  (bind _arrayweaponpool (Variables|Default|GetArrayWeaponPool))
  (for (_array_element _array_index) (Variables|Default|GetArrayWeaponPool)
    (if (== (Utilities|GetClass _array_element) CWeapon)
      (Variables|Default|SetOutWeapon (Utilities|Array|Get(acopy) _arrayweaponpool _array_index))
      (Utilities|Array|RemoveIndex _arrayweaponpool _array_index)
      (return true (Variables|Default|GetOutWeapon))))
  (return false 0))

(fn FAddAmmoPool
  (params (OAmmo :type BP%20Ammo%20Base%20Kostin%20Object%20Reference))
  (Utilities|Array|Add (Variables|Default|GetArrayAmmoPool) OAmmo)
  (bind _returnvalue (Actor|GetActorOfClass "/Game/Core/BP_Kostin/Character/NPC/BP_ActorNULL.BP_ActorNULL_C"))
  (Transformation|AttachActorToActor OAmmo _returnvalue "None" "SnapToTarget" "SnapToTarget" "SnapToTarget" true))

(fn FSearchAmmoPool
  (params (CAmmoClass :type BP%20Ammo%20Base%20Kostin%20Class%20Reference))
  (bind _arrayammopool (Variables|Default|GetArrayAmmoPool))
  (for (_array_element _array_index) (Variables|Default|GetArrayAmmoPool)
    (if (== (Utilities|GetClass _array_element) CAmmoClass)
      (Variables|Default|SetOutAmmo (Utilities|Array|Get(acopy) _arrayammopool _array_index))
      (Utilities|Array|RemoveIndex _arrayammopool _array_index)
      (return true (Variables|Default|GetOutAmmo))))
  (return false 0))