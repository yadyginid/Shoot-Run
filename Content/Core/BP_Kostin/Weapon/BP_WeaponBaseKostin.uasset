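; BP_WeaponBaseKostin is a weapon Blueprint, named as a base, whose Fire event plays a fire animation montage on its instigator Character.
; The PlayAni flag blocks repeat triggers until a Delay matching the returned montage length ends.
; An invalid montage or failed cast prints an error, and the invalid-montage path leaves PlayAni set, blocking later Fire calls.
; It contains no projectile, trace or damage logic.
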(event Custom|Fire
  (bind _animfire (Variables|Default|GetAnimFire))
  ;[0.15 0.15 0.15 0.5] Play Anim Fire
  (bind _ascharacter (Utilities|Casting|CastToCharacter (Game|GetInstigator))
    (:then
      (if (not (Variables|Default|GetbPlayAni))
        (Variables|Default|SetbPlayAni true)
        (Utilities|IsValid _animfire
          (:Is%20Valid
            (bind _returnvalue (Animation|PlayAnimMontage _ascharacter _animfire 1.0 "None"))
            (Utilities|FlowControl|Delay _returnvalue)
            (Variables|Default|SetbPlayAni false))
          (:Is%20Not%20Valid
            (Development|PrintString "Error Anim is not valid")))))
    (:CastFailed
      (Development|PrintString "Error Cast Failed"))))

(event EventBeginPlay)

(event Collision|EventActorBeginOverlap
  (params (OtherActor :type Actor%20Object%20Reference)))

(event EventTick
  (params (DeltaSeconds :type Float%20%28single-precision%29)))

(fn ConstructionScript)