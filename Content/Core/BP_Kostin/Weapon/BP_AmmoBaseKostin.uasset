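; BP_AmmoBaseKostin is a base ammo projectile that damages what its sphere overlaps and then hands itself to the game mode's ammo pool for reuse.
; On overlap it ignores itself and its owner, clears its active flag, returns to the pool, deactivates its projectile movement and applies damage.
; The game mode reference is cached at BeginPlay, and the applied damage is printed on screen for debugging.
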(event OnComponentBeginOverlap(Sphere)
  (params (OverlappedComponent :type Primitive%20Component%20Object%20Reference) (OtherActor :type Actor%20Object%20Reference) (OtherComp :type Primitive%20Component%20Object%20Reference) (OtherBodyIndex :type Integer) (bFromSweep :type Boolean) (SweepResult :type Hit%20Result%20Structure%20%28by%20ref%29))
  (bind _returnvalue (Components|GetOwner OverlappedComponent))
  (if (!= _returnvalue OtherActor)
    (if (!= (Components|GetOwner _returnvalue) OtherActor)
      (if (Variables|Default|GetisActive)
        (Variables|Default|SetisActive false)
        (Default|FAddAmmoPool (Variables|Default|GetAs%20BP%20Game%20Mode%20Kostin) self)
        (Components|Activation|Deactivate (Variables|Default|GetProjectileMovement))
        (bind _returnvalue_2 (Game|Damage|ApplyDamage OtherActor (Math|Conversions|ToFloat(Integer) (Variables|Default|GetDamage)) 0 0))
        (Development|PrintString (Utilities|String|ToString(Float) _returnvalue_2) true true "(R=1.000000,G=0.000000,B=0.131718,A=1.000000)")))))

(event EventBeginPlay
  (bind _asbp_game_mode_kostin (Utilities|Casting|CastToBP_GameModeKostin (Game|GetGameMode)))
  (Variables|Default|SetAs%20BP%20Game%20Mode%20Kostin _asbp_game_mode_kostin))

(fn ConstructionScript)