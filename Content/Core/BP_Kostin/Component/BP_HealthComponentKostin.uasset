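; Actor component that tracks health and death for its owner, caching the starting Health as MaxHealth on BeginPlay.
; It binds to the owner's OnTakeAnyDamage and routes each hit into Damage, which subtracts health while Alive, calls UpdateHeath and prints the value for debugging.
; At zero or below it clears Alive and calls EventDead, while the Dead function itself is an empty stub.
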(event Custom|CustomEvent
  (params (DamagedActor :type Actor%20Object%20Reference) (Damage :type Float%20%28single-precision%29) (DamageType :type Damage%20Type%20Object%20Reference) (InstigatedBy :type Controller%20Object%20Reference) (DamageCauser :type Actor%20Object%20Reference))
  (CallFunction|Damage Damage))

(event EventBeginPlay
  (Variables|Default|SetMaxHealth (Variables|Default|GetHealth))
  (EventDispatchers|BindEventtoOnTakeAnyDamage (Components|GetOwner) (delegate Custom|CustomEvent)))

(event EventTick
  (params (DeltaSeconds :type Float%20%28single-precision%29)))

(fn Damage
  (params (Damage :type Float%20%28double-precision%29))
  (if (Variables|Default|GetAlive)
    (bind _output_get (Variables|Default|SetHealth (- (Variables|Default|GetHealth) Damage)))
    (Default|CallUpdateHeath)
    (Development|PrintString (Utilities|String|Append "Health" (Utilities|String|ToString(Float) _output_get)))
    (if (<= (Variables|Default|GetHealth) 0.0)
      (Variables|Default|SetAlive false)
      (Default|CallEventDead))))

(fn Dead)