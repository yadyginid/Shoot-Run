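; Actor component that gives a zombie character a melee attack that damages BP_CharacterBaseKostin actors.
; On BeginPlay it adds a small sphere to the owner's right-hand socket, applying damage on overlap while attacking and not dead.
; ZombieAttack plays the attack montage and sets a timer for its length, while StopAttack and FisDead set the gating flags.
; The left-hand sphere's creation and overlap binding are present but never run.
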(event Custom|onSphere1BeginOverlap
  (params (OverlappedComponent :type Primitive%20Component%20Object%20Reference) (OtherActor :type Actor%20Object%20Reference) (OtherComp :type Primitive%20Component%20Object%20Reference) (OtherBodyIndex :type Integer) (bFromSweep :type Boolean) (SweepResult :type Hit%20Result%20Structure%20%28by%20ref%29))
  (if (Variables|Default|GetisAttack)
    (if (not (Variables|Default|GetisDead))
      (bind _asbp_character_base_kostin (Utilities|Casting|CastToBP_CharacterBaseKostin OtherActor))
      (Game|Damage|ApplyDamage _asbp_character_base_kostin (Variables|Default|GetBase%20Damage) 0 0))))

(event Custom|onSphere2BeginOverlap
  (params (OverlappedComponent :type Primitive%20Component%20Object%20Reference) (OtherActor :type Actor%20Object%20Reference) (OtherComp :type Primitive%20Component%20Object%20Reference) (OtherBodyIndex :type Integer) (bFromSweep :type Boolean) (SweepResult :type Hit%20Result%20Structure%20%28by%20ref%29))
  (if (Variables|Default|GetisAttack)
    (if (not (Variables|Default|GetisDead))
      (bind _asbp_character_base_kostin (Utilities|Casting|CastToBP_CharacterBaseKostin OtherActor))
      (Game|Damage|ApplyDamage _asbp_character_base_kostin (Variables|Default|GetBase%20Damage) 0 0))))

(event EventBeginPlay
  (CallFunction|SpawnZombieSphere)
  (Collision|BindEventtoOnComponentBeginOverlap (Variables|Default|GetSphere1) (delegate Custom|onSphere1BeginOverlap)))

(fn SpawnZombieSphere
  (bind _returnvalue (Components|GetOwner))
  (bind _returnvalue_2 (Game|AddComponentbyClass _returnvalue "/Script/Engine.SphereComponent" false (Transformation|GetActorTransform _returnvalue)))
  (bind _output_get (Variables|Default|SetSphere1 _returnvalue_2))
  (Components|Sphere|SetSphereRadius _output_get 8.0 true)
  (bind _ascharacter (Utilities|Casting|CastToCharacter (Components|GetOwner)))
  (Transformation|AttachComponentToComponent (Variables|Default|GetSphere1) (Variables|/Script/Engine.Character|GetMesh _ascharacter) "RightHandSocket" "SnapToTarget" "SnapToTarget" "SnapToTarget" true))

(fn ZombieAttack
  (if (not (Variables|Default|GetisDead))
    (if (not (Variables|Default|GetisAttack))
      (Variables|Default|SetisAttack true)
      (bind _ascharacter (Utilities|Casting|CastToCharacter (Components|GetOwner)))
      (bind _returnvalue (Animation|PlayAnimMontage _ascharacter "/Game/Core/BP_Kostin/Player/Animation/Zombie/AM_Zombie_Attack.AM_Zombie_Attack" 1.0 "None"))
      (Utilities|Time|SetTimerbyEvent (EventDispatchers|CreateEvent :!event StopAttack) _returnvalue))))

(fn StopAttack
  (Variables|Default|SetisAttack false))

(fn FisDead
  (Variables|Default|SetisDead true))