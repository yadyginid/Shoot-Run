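; NPC character Blueprint that gives its weapon to the player on first interaction.
; BeginPlay spawns the weapon through its weapon component and caches the game mode.
; BPIAction clears a Dialog flag, adds the weapon to the game mode's pool and passes its class to the player via CallActionNPC; later interactions only print a refusal.
; NPCRotation turns the actor to face the player, though nothing here calls it.
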(event EventBeginPlay
  (Default|SpawnWeapon (Variables|Default|GetBP_WeaponComponentKostin))
  (bind _asbp_game_mode_kostin (Utilities|Casting|CastToBP_GameModeKostin (Game|GetGameMode)))
  (Variables|Default|SetAs%20BP%20Game%20Mode%20Kostin _asbp_game_mode_kostin))

(event EventBPIAction
  (bind _bp_weaponcomponentkostin (Variables|Default|GetBP_WeaponComponentKostin))
  (bind _weapon (Variables|/Game/Core/BP_Kostin/Component/BP_WeaponComponentKostin.BP_WeaponComponentKostin_C|GetWeapon _bp_weaponcomponentkostin))
  (if (Variables|Default|GetDialog)
    (Development|PrintString "Привет, вот тебе мое оружие!")
    (Variables|Default|SetDialog false)
    (Utilities|IsValid _weapon
      (:Is%20Valid
        (Default|FAddWeaponPool (Variables|Default|GetAs%20BP%20Game%20Mode%20Kostin) _weapon)
        (bind _asbp_character_base_kostin (Utilities|Casting|CastToBP_CharacterBaseKostin (Game|GetPlayerCharacter 0)))
        (Default|CallActionNPC _asbp_character_base_kostin (Variables|/Game/Core/BP_Kostin/Component/BP_WeaponComponentKostin.BP_WeaponComponentKostin_C|GetWeapon%20Class (Variables|Default|GetBP_WeaponComponentKostin)))))
    (else
      (Development|PrintString "Я уже отдал тебе свое оружие! Что тебе еще от меня надо?"))))

(fn ConstructionScript
  (|CallParentFunction))

(fn NPCRotation
  (Transformation|SetActorRotation (Math|Rotator|FindLookatRotation (Transformation|GetActorLocation) (Transformation|GetActorLocation (Game|GetPlayerCharacter 0))))
  (return))