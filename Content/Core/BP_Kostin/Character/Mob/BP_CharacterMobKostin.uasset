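; Team-based mob character built from team, health and weapon components.
; On BeginPlay it sets its team, binds to the health component's death event, spawns a weapon and caches the game mode.
; Death calls Dead and returns the weapon to the game mode's pool.
; BPIAction triggers SetWeapon on an ally AI controller and prints an enemy label for non-zero teams; animation and movement logic is stubbed or disconnected.
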(event Custom|Event%20NPC%20Animation
  (if true
    _))

(event Custom|CustomEvent
  ;[0.15 0.15 0.15 0.5] Comment
  (CallFunction|Dead)
  (Default|FAddWeaponPool (Variables|Default|GetAs%20BP%20Game%20Mode%20Kostin) (Variables|/Game/Core/BP_Kostin/Component/BP_WeaponComponentKostin.BP_WeaponComponentKostin_C|GetWeapon (Variables|Default|GetBP_WeaponComponentKostin))))

(event EventBeginPlay
  ;[0.15 0.15 0.15 0.5] Comment
  (Default|UpdateNumTeam (Variables|Default|GetBP_TeamComponentKostin) (Variables|Default|GetNumTeam))
  (EventDispatchers|BindEventtoEventDead (Variables|Default|GetBP_HealthComponentKostin) (delegate Custom|CustomEvent))
  (Default|SpawnWeapon (Variables|Default|GetBP_WeaponComponentKostin))
  (bind _asbp_game_mode_kostin (Utilities|Casting|CastToBP_GameModeKostin (Game|GetGameMode)))
  (Variables|Default|SetAs%20BP%20Game%20Mode%20Kostin _asbp_game_mode_kostin))

(event Collision|EventActorBeginOverlap
  (params (OtherActor :type Actor%20Object%20Reference))
  (|CallParentFunction OtherActor) ; This node is disabled and will not be called.\nDrag off pins to build functionality.
)

(event EventBPIAction
  ;[0.15 0.15 0.15 0.5] Comment
  (bind _asbp_aicontroller_ally_kostin (Utilities|Casting|CastToBP_AIControllerAllyKostin (Pawn|GetController))
    (:then
      (Default|SetWeapon _asbp_aicontroller_ally_kostin))
    (:CastFailed
      _))
  (if (== (Variables|Default|GetNumTeam) 0)
    (bind _outactors (Actor|GetAllActorsOfClass "BP_CharacterMobKostin_C"))
    (bind _array_element (Utilities|Array|ForEachLoopwithBreak _outactors)
      (:LoopBody
        (if (== (Variables|BP_CharacterMobKostin_C|GetNumTeam _array_element) 0)
          _)))
    (else
      (Development|PrintString "Враг"))))

(fn ConstructionScript
  (|CallParentFunction))

(fn NPCRotation)