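; BP_CharacterZMobKostin is a mob character that handles its own death.
; On BeginPlay it binds OnDead to the death event of its health component.
; OnDead sets the IsLive key in its controller's Blackboard to false, then calls Dead.
; Dead plays the AM_Dead montage and uses the returned duration as the actor's life span, so the mob is destroyed as the animation ends.
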(event Custom|OnDead
  (AI|Components|Blackboard|SetValueasBool (AI|GetBlackboard (Pawn|GetController)) (Variables|Default|GetisLive) false)
  (CallFunction|Dead))

(event EventBeginPlay
  (EventDispatchers|BindEventtoEventDead (Variables|Default|GetBP_HealthComponentKostin) (delegate Custom|OnDead)))

(event Collision|EventActorBeginOverlap
  (params (OtherActor :type Actor%20Object%20Reference))
  (|CallParentFunction OtherActor) ; This node is disabled and will not be called.\nDrag off pins to build functionality.
)

(event EventTick
  (params (DeltaSeconds :type Float%20%28single-precision%29))
  (|CallParentFunction DeltaSeconds) ; This node is disabled and will not be called.\nDrag off pins to build functionality.
)

(fn ConstructionScript
  (|CallParentFunction))

(fn Dead
  (bind _returnvalue (Animation|PlayAnimMontage "/Game/Core/Blueprints/Player/Animations/AM_Dead.AM_Dead" 1.0 "None"))
  (Actor|SetLifeSpan _returnvalue))