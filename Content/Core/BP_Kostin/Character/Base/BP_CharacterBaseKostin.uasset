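; Base character Blueprint that provides health-gated movement with sprinting, weapon spawning, interaction and death.
; Weapon and health components drive it: an NPC action event equips and stores a new weapon class, and death plays a montage whose length sets the actor's lifespan.
; Interact line-traces forward to message BPI_ActionKostin actors.
; A separate fan of visibility traces, swept across several vertical offsets, swaps the mesh material of characters it hits.
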(event Custom|onActionNPC
  (params (WeaponClass :type BP%20Weapon%20Base%20Kostin%20Class%20Reference))
  (bind _bp_weaponcomponentkostin (Variables|Default|GetBP_WeaponComponentKostin))
  (bind _output_get (Variables|/Game/Core/BP_Kostin/Component/BP_WeaponComponentKostin.BP_WeaponComponentKostin_C|SetWeapon%20Class (Variables|Default|GetBP_WeaponComponentKostin) WeaponClass))
  (Default|SpawnWeapon _bp_weaponcomponentkostin)
  (Utilities|IsValid (Variables|/Game/Core/BP_Kostin/Component/BP_WeaponComponentKostin.BP_WeaponComponentKostin_C|GetWeapon _bp_weaponcomponentkostin)
    (:Is%20Valid
      (bind _returnvalue (Utilities|Array|Add (Variables|/Game/Core/BP_Kostin/Component/BP_WeaponComponentKostin.BP_WeaponComponentKostin_C|GetAWeapon (Variables|Default|GetBP_WeaponComponentKostin)) _output_get))
      (Variables|/Game/Core/BP_Kostin/Component/BP_WeaponComponentKostin.BP_WeaponComponentKostin_C|SetNumWeapon (Variables|Default|GetBP_WeaponComponentKostin) _returnvalue))))

(event Custom|OnDead
  (CallFunction|Dead))

(event EventBeginPlay
  (Default|SpawnWeapon (Variables|Default|GetBP_WeaponComponentKostin))
  (EventDispatchers|BindEventtoActionNPC (delegate Custom|onActionNPC))
  (EventDispatchers|BindEventtoEventDead (Variables|Default|GetBP_HealthComponentKostin) (delegate Custom|OnDead))
  (bind _asbp_game_mode_kostin (Utilities|Casting|CastToBP_GameModeKostin (Game|GetGameMode)))
  (Variables|Default|SetGameMode _asbp_game_mode_kostin)
  (Default|CallLoaded))

(event Collision|EventActorBeginOverlap
  (params (OtherActor :type Actor%20Object%20Reference)))

(event EventTick
  (params (DeltaSeconds :type Float%20%28single-precision%29)))

(fn ConstructionScript)

(fn Interact
  (bind _arrow1 (Variables|Default|GetArrow1))
  (bind _returnvalue (Transformation|GetWorldLocation _arrow1))
  (if (Variables|/Game/Core/BP_Kostin/Component/BP_HealthComponentKostin.BP_HealthComponentKostin_C|GetAlive (Variables|Default|GetBP_HealthComponentKostin))
    (bind _outhit (Collision|LineTraceByChannel _returnvalue (+ _returnvalue (* (Math|Vector|GetForwardVector _arrow1) 300)) "TraceTypeQuery3" true 0 "ForDuration" true "(R=0.000000,G=0.033624,B=1.000000,A=1.000000)" "(R=0.988398,G=0.000000,B=1.000000,A=1.000000)"))
    (if (Utilities|DoesObjectImplementInterface (.HitActor (Collision|BreakHitResult _outhit)) "/Game/Core/BP_Kostin/Interfaces/BPI_ActionKostin.BPI_ActionKostin_C")
      (Class|BPIActionKostin|BPIAction(Message) (.HitActor (Collision|BreakHitResult _outhit))))))

(fn Dead
  (bind _returnvalue (Animation|PlayAnimMontage "/Game/Core/Blueprints/Player/Animations/AM_Dead.AM_Dead" 1.0 "None"))
  (Actor|SetLifeSpan _returnvalue))

(fn VisLineTrace
  (params (A_Y :type Float%20%28double-precision%29) (A_Z :type Float%20%28double-precision%29))
  (bind _self self)
  (bind _arrow2 (Variables|Default|GetArrow2 _self))
  (bind _returnvalue (Transformation|GetSocketLocation _arrow2 "None"))
  (bind _outhit (Collision|LineTraceByChannel _returnvalue (+ _returnvalue (* (Math|Vector|RotateVector (Math|Vector|MakeVector 1.0 A_Y A_Z) (.rotation (Transformation|GetActorTransform))) (Variables|Default|GetVisDistanse))) "TraceTypeQuery1" false 0 "ForDuration" true "(R=0.905026,G=0.000000,B=1.000000,A=1.000000)" "(R=0.000000,G=0.670709,B=1.000000,A=1.000000)"))
  (bind _ascharacter (Utilities|Casting|CastToCharacter (.HitActor (Collision|BreakHitResult _outhit))))
  (Rendering|Material|SetMaterial (Variables|/Script/Engine.Character|GetMesh _ascharacter) 0 "/Engine/VREditor/UI/ArrowMaterial.ArrowMaterial")
  (return))

(fn Move
  (params (X :type Float%20%28double-precision%29) (Y :type Float%20%28double-precision%29))
  (if (Variables|/Game/Core/BP_Kostin/Component/BP_HealthComponentKostin.BP_HealthComponentKostin_C|GetAlive (Variables|Default|GetBP_HealthComponentKostin))
    (if (Math|Boolean|ANDBoolean (> Y 0.8) (Variables|Default|GetbSprint) true)
      (Variables|/Script/Engine.CharacterMovementComponent|SetMaxWalkSpeed (Variables|Character|GetCharacterMovement) (Variables|Default|GetfMaxWalkSpeedSprint))
      (else
        (Variables|/Script/Engine.CharacterMovementComponent|SetMaxWalkSpeed (Variables|Character|GetCharacterMovement) (Variables|Default|GetfMaxWalkSpeed))))
    (Pawn|Input|AddMovementInput (Transformation|GetActorForwardVector) Y false)
    (Pawn|Input|AddMovementInput (Transformation|GetActorRightVector) X false)))

(fn ArrVisLineTrace
  (bind _vismaxtrace (Variables|Default|GetVisMaxTrace))
  (bind _returnvalue (/ _vismaxtrace 2))
  (for _array_element (Variables|Default|GetArrayVisZAxis)
    (Variables|Default|SetVisZAxis _array_element)
    (for _index (range 0 _returnvalue)
      (CallFunction|VisLineTrace (* _index (/ 1 (Math|Conversions|ToFloat(Integer) _returnvalue))) (Variables|Default|GetVisZAxis))
      (CallFunction|VisLineTrace (* (* _index (/ 1 (Math|Conversions|ToFloat(Integer) _returnvalue))) -1) (Variables|Default|GetVisZAxis)))))