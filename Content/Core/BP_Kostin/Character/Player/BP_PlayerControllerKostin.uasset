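; Player controller that turns player input into actions on the controlled BP_CharacterBaseKostin.
; On BeginPlay it adds the IMC_PlayerMovement mapping context and caches the cast pawn once.
; Input events drive movement, sprint, interaction and a line-trace visual on key 1, and call the character's weapon component to fire or switch weapons.
; Look, fire and weapon switching require the health component's Alive flag; move, sprint and interact do not check it.
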(event Input|EnhancedActionEvents|EnhancedInputActionIA_Sprint
  (params (ActionValue :type Boolean) (ElapsedSeconds :type Float%20%28double-precision%29) (TriggeredSeconds :type Float%20%28double-precision%29) (InputAction :type Input%20Action%20Object%20Reference :default "/Game/Core/Input/Actions/IA_Sprint.IA_Sprint"))
  (bind _as_bp_character_base_kostin (Variables|Default|GetAs%20BP%20Character%20Base%20Kostin))
  (bind _as_bp_character_base_kostin_2 (Variables|Default|GetAs%20BP%20Character%20Base%20Kostin))
  ;[0.15 0.15 0.15 0.5] Sprint
  (:Started
    (Utilities|IsValid _as_bp_character_base_kostin_2
      (:Is%20Valid
        (Variables|/Game/Core/BP_Kostin/Character/Base/BP_CharacterBaseKostin.BP_CharacterBaseKostin_C|SetbSprint _as_bp_character_base_kostin true))))
  (:Completed
    (Utilities|IsValid _as_bp_character_base_kostin_2
      (:Is%20Valid
        (Variables|/Game/Core/BP_Kostin/Character/Base/BP_CharacterBaseKostin.BP_CharacterBaseKostin_C|SetbSprint _as_bp_character_base_kostin false)))))

(event Input|EnhancedActionEvents|EnhancedInputActionIA_Move
  (params (ActionValue :type Vector%202D%20Structure) (ElapsedSeconds :type Float%20%28double-precision%29) (TriggeredSeconds :type Float%20%28double-precision%29) (InputAction :type Input%20Action%20Object%20Reference :default "/Game/Core/Input/Actions/IA_Move.IA_Move"))
  ;[0.15 0.15 0.15 0.5] move
  (Default|Move (Variables|Default|GetAs%20BP%20Character%20Base%20Kostin) (.x ActionValue) (.y ActionValue)))

(event Input|EnhancedActionEvents|EnhancedInputActionIA_Look
  (params (ActionValue :type Vector%202D%20Structure) (ElapsedSeconds :type Float%20%28double-precision%29) (TriggeredSeconds :type Float%20%28double-precision%29) (InputAction :type Input%20Action%20Object%20Reference :default "/Game/Core/Input/Actions/IA_Look.IA_Look"))
  (bind _as_bp_character_base_kostin (Variables|Default|GetAs%20BP%20Character%20Base%20Kostin))
  (bind _as_bp_character_base_kostin_2 (Variables|Default|GetAs%20BP%20Character%20Base%20Kostin))
  ;[0.15 0.15 0.15 0.5] Look
  (Utilities|IsValid _as_bp_character_base_kostin_2
    (:Is%20Valid
      (if (Variables|/Game/Core/BP_Kostin/Component/BP_HealthComponentKostin.BP_HealthComponentKostin_C|GetAlive (Variables|/Game/Core/BP_Kostin/Character/Base/BP_CharacterBaseKostin.BP_CharacterBaseKostin_C|GetBP_HealthComponentKostin _as_bp_character_base_kostin_2))
        (Pawn|Input|AddControllerYawInput _as_bp_character_base_kostin (.x ActionValue))
        (Pawn|Input|AddControllerPitchInput _as_bp_character_base_kostin (.y ActionValue))))))

(event Input|EnhancedActionEvents|EnhancedInputActionIA_Fire
  (params (ActionValue :type Boolean) (ElapsedSeconds :type Float%20%28double-precision%29) (TriggeredSeconds :type Float%20%28double-precision%29) (InputAction :type Input%20Action%20Object%20Reference :default "/Game/Core/Input/Actions/IA_Fire.IA_Fire"))
  ;[0.15 0.15 0.15 0.5] Fire
  (Utilities|IsValid (Variables|/Game/Core/BP_Kostin/Component/BP_WeaponComponentKostin.BP_WeaponComponentKostin_C|GetWeapon (Variables|/Game/Core/BP_Kostin/Character/Base/BP_CharacterBaseKostin.BP_CharacterBaseKostin_C|GetBP_WeaponComponentKostin (Variables|Default|GetAs%20BP%20Character%20Base%20Kostin)))
    (:Is%20Valid
      (if (Variables|/Game/Core/BP_Kostin/Component/BP_HealthComponentKostin.BP_HealthComponentKostin_C|GetAlive (Variables|/Game/Core/BP_Kostin/Character/Base/BP_CharacterBaseKostin.BP_CharacterBaseKostin_C|GetBP_HealthComponentKostin (Variables|Default|GetAs%20BP%20Character%20Base%20Kostin)))
        (Default|FireWeapon (Variables|/Game/Core/BP_Kostin/Character/Base/BP_CharacterBaseKostin.BP_CharacterBaseKostin_C|GetBP_WeaponComponentKostin (Variables|Default|GetAs%20BP%20Character%20Base%20Kostin)))))
    (:Is%20Not%20Valid
      (Development|PrintString "No Weapon"))))

(event Input|EnhancedActionEvents|EnhancedInputActionIA_Interact
  (params (ActionValue :type Boolean) (ElapsedSeconds :type Float%20%28double-precision%29) (TriggeredSeconds :type Float%20%28double-precision%29) (InputAction :type Input%20Action%20Object%20Reference :default "/Game/Core/Input/Actions/IA_Interact.IA_Interact"))
  ;[0.15 0.15 0.15 0.5] Interact
  (Default|Interact (Variables|Default|GetAs%20BP%20Character%20Base%20Kostin)))

(event EventBeginPlay
  (bind _self self)
  (bind _returnvalue (PlayerController|LocalPlayerSubsystems|GetEnhancedInputLocalPlayerSubsystem _self))
  (Utilities|IsValid _returnvalue
    (:Is%20Valid
      (Input|AddMappingContext _returnvalue "/Game/Core/Input/IMC_PlayerMovement.IMC_PlayerMovement" 0 "(bIgnoreAllPressedKeysUntilRelease=True,bForceImmediately=False,bNotifyUserSettings=False)")
      (bind _asbp_character_base_kostin (Utilities|Casting|CastToBP_CharacterBaseKostin (Pawn|GetControlledPawn)))
      (Utilities|IsValid _asbp_character_base_kostin
        (:Is%20Valid
          (Variables|Default|SetAs%20BP%20Character%20Base%20Kostin _asbp_character_base_kostin))))))

(event Input|ActionEvents|InputActionNextWeapon
  (params (Key :type Key%20Structure :default "None"))
  ;[0.15 0.15 0.15 0.5] NextWeapon
  (:Pressed
    (if (Variables|/Game/Core/BP_Kostin/Component/BP_HealthComponentKostin.BP_HealthComponentKostin_C|GetAlive (Variables|/Game/Core/BP_Kostin/Character/Base/BP_CharacterBaseKostin.BP_CharacterBaseKostin_C|GetBP_HealthComponentKostin (Variables|Default|GetAs%20BP%20Character%20Base%20Kostin)))
      (Default|NextWeapon (Variables|/Game/Core/BP_Kostin/Character/Base/BP_CharacterBaseKostin.BP_CharacterBaseKostin_C|GetBP_WeaponComponentKostin (Variables|Default|GetAs%20BP%20Character%20Base%20Kostin))))))

(event Input|ActionEvents|InputActionPrevWeapon
  (params (Key :type Key%20Structure :default "None"))
  ;[0.15 0.15 0.15 0.5] PrevWeapon
  (:Pressed
    (if (Variables|/Game/Core/BP_Kostin/Component/BP_HealthComponentKostin.BP_HealthComponentKostin_C|GetAlive (Variables|/Game/Core/BP_Kostin/Character/Base/BP_CharacterBaseKostin.BP_CharacterBaseKostin_C|GetBP_HealthComponentKostin (Variables|Default|GetAs%20BP%20Character%20Base%20Kostin)))
      (Default|PrevWeapon (Variables|/Game/Core/BP_Kostin/Character/Base/BP_CharacterBaseKostin.BP_CharacterBaseKostin_C|GetBP_WeaponComponentKostin (Variables|Default|GetAs%20BP%20Character%20Base%20Kostin))))))

(event Input|KeyboardEvents|1
  (params (Key :type Key%20Structure :default "None"))
  ;[0.15 0.15 0.15 0.5] visuality effect
  (:Pressed
    (Default|ArrVisLineTrace (Variables|Default|GetAs%20BP%20Character%20Base%20Kostin))))

(fn ConstructionScript)